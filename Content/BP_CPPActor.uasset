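; BP_CPPActor is an actor Blueprint that exercises C++-to-Blueprint event hooks with debug output.
; BeginPlay prints and logs startup text, and Tick prints a message every frame.
; PlayFireEffectsBPImplem and PlayFireEffectsBPNativeEv print tagged Radius values; the latter adds ComponentBaseForBlueprint's Diameter and prints the count of OpeningEngine actors.
; A loop over those actors and a StartOptimization call are left unconnected and never run.
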(event EventBeginPlay
  (Development|PrintString "START")
  (Utilities|String|LogString "Hello"))

(event Collision|EventActorBeginOverlap
  (params (OtherActor :type Actor%20Object%20Reference)))

(event EventTick
  (params (DeltaSeconds :type Float%20%28single-precision%29))
  (Development|PrintString "BP Tick"))

(event EventPlayFireEffectsBPImplem
  (Development|PrintString (Utilities|String|Append (Utilities|String|MakeLiteralString "BP: Implementable ") (Utilities|String|ToString(Float) (Variables|Default|GetRadius)))))

(event EventPlayFireEffectsBPNativeEv
  (Development|PrintString (Utilities|String|Append (Utilities|String|MakeLiteralString "BP: Native ") (Utilities|String|ToString(Float) (Variables|Default|GetRadius)) (Utilities|String|ToString(Float) (Variables|/Script/LotusTestBed.ComponentBaseForBlueprint|GetDiameter (Variables|Default|GetComponentBaseForBlueprint)))))
  (bind _outactors (Actor|GetAllActorsOfClass "/Script/LotusTestBed.OpeningEngine"))
  (Development|PrintString (Utilities|String|ToString(Integer) (Utilities|Array|Length _outactors))))

(fn ConstructionScript)