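; Dynamic mesh actor that shows a flat box slab with a movable hole cut through it using Geometry Script.
; The construction script builds the uncut slab.
; MoveHole rebuilds it, boolean-subtracts a temporary compute-mesh box at an XY position clamped to the slab bounds, prints that position and releases compute meshes.
; MoveHoleDebug runs MoveHole with the HolePositionDebug variable, and the event graph is unused.
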(event EventBeginPlay)

(event Collision|EventActorBeginOverlap
  (params (OtherActor :type Actor%20Object%20Reference)))

(event EventTick
  (params (DeltaSeconds :type Float%20%28single-precision%29)))

(fn ConstructionScript
  (bind _returnvalue (DynamicMeshComponent|GetDynamicMesh (Variables|DynamicMeshActor|GetDynamicMeshComponent)))
  (bind _returnvalue_2 (DynamicMesh|Reset _returnvalue))
  (Class|GeometryScriptLibraryMeshPrimitiveFunctions|AppendBox :TargetMesh _returnvalue_2 :DimensionX 4e+02 :DimensionY 4e+02 :DimensionZ 2e+01 :Debug 0))

(fn MoveHole
  (params (Test :type Vector))
  (bind _returnvalue (Math|Float|Clamp(Float) (.x Test) -2e+02 2e+02))
  (bind _returnvalue_2 (Math|Float|Clamp(Float) (.y Test) -2e+02 2e+02))
  (bind _returnvalue_3 (DynamicMeshComponent|GetDynamicMesh (Variables|DynamicMeshActor|GetDynamicMeshComponent)))
  (bind _returnvalue_4 (DynamicMesh|Reset _returnvalue_3))
  (bind _returnvalue_5 (Class|GeometryScriptLibraryMeshPrimitiveFunctions|AppendBox :TargetMesh _returnvalue_4 :DimensionX 4e+02 :DimensionY 4e+02 :DimensionZ 2e+01 :Debug 0))
  (bind _returnvalue_6 (DynamicMeshActor|AllocateComputeMesh))
  (bind _returnvalue_7 (Class|GeometryScriptLibraryMeshPrimitiveFunctions|AppendBox :TargetMesh _returnvalue_6 :Transform (Math|Transform|MakeTransform (Math|Vector|MakeVector _returnvalue _returnvalue_2 0.0) "0, 0, 0" "1.000000,1.000000,1.000000") :Debug 0))
  (GeometryScript|Booleans|ApplyMeshBoolean :TargetMesh _returnvalue_5 :ToolMesh _returnvalue_7 :Operation "Subtract" :Debug 0)
  (Development|PrintString (Utilities|String|Append (Utilities|String|Append (Utilities|String|Append (Utilities|String|MakeLiteralString "Val ") (Utilities|String|ToString(Float) _returnvalue)) " : ") (Utilities|String|ToString(Float) _returnvalue_2)))
  (DynamicMeshActor|ReleaseAllComputeMeshes))

(fn MoveHoleDebug
  (CallFunction|MoveHole (Variables|Debug|GetHolePositionDebug)))