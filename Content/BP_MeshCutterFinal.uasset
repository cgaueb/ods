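; Geometry Script actor that subtracts a cutter static mesh from a copy of the Cutted actor's mesh.
; Initialize, also run on construction, rebuilds the dynamic mesh from Cutted with its relative transform and stores Position, or appends a sphere box if Cutted is invalid.
; Cut calls Initialize first, so cuts do not accumulate, then applies a boolean subtract using a pooled compute mesh offset by Position.
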(event EventBeginPlay)

(event Collision|EventActorBeginOverlap
  (params (OtherActor :type Actor%20Object%20Reference)))

(event EventTick
  (params (DeltaSeconds :type Float%20%28single-precision%29)))

(fn ConstructionScript
  (CallFunction|Initialize))

(fn Cut
  (params (Transform :type Transform) (Cutter :type Static%20Mesh%20Object%20Reference))
  (CallFunction|Initialize)
  (bind _returnvalue (DynamicMeshComponent|GetDynamicMesh (Variables|DynamicMeshActor|GetDynamicMeshComponent)))
  (bind _returnvalue_2 (DynamicMeshActor|AllocateComputeMesh))
  (if true
    (bind _returnvalue_3 (GeometryScript|StaticMesh|CopyMeshFromStaticMesh :FromStaticMeshAsset Cutter :ToDynamicMesh _returnvalue_2 :Debug 0)
      (:Success
        _))
    (else
      (Class|GeometryScriptLibraryMeshPrimitiveFunctions|AppendBox :TargetMesh _returnvalue_2 :Debug 0)))
  (GeometryScript|Booleans|ApplyMeshBoolean :TargetMesh _returnvalue :ToolMesh _returnvalue_3 :ToolTransform (Math|Transform|ComposeTransforms Transform (Math|Transform|MakeTransform (Variables|Default|GetPosition))) :Operation "Subtract" :Debug 0)
  (DynamicMeshActor|ReleaseAllComputeMeshes))

(fn Initialize
  (bind _returnvalue (DynamicMeshComponent|GetDynamicMesh (Variables|DynamicMeshActor|GetDynamicMeshComponent)))
  (bind _cutted (Variables|Default|GetCutted)
    (:then
      (bind _returnvalue_2 (DynamicMesh|Reset _returnvalue))
      (bind _returnvalue_3 (GeometryScript|Scene|CopyMeshfromComponent :Component (Variables|/Script/Engine.StaticMeshActor|GetStaticMeshComponent _cutted) :ToDynamicMesh _returnvalue_2 :Debug 0)
        (:Failure
          (Development|PrintText "BP_MeshCutterFinal: Error in Copying" true true "(R=1.000000,G=0.026276,B=0.000000,A=1.000000)"))
        (:Success
          (GeometryScript|Transforms|TransformMesh _returnvalue_3 (Transformation|GetRelativeTransform (Variables|/Script/Engine.StaticMeshActor|GetStaticMeshComponent _cutted)) 0)
          (Variables|Default|SetPosition (.location (Math|Transform|ComposeTransforms (Transformation|GetRelativeTransform (Variables|/Script/Engine.StaticMeshActor|GetStaticMeshComponent _cutted)) (Math|Transform|MakeTransform "0, 0, 0")))))))
    (:else
      (bind _returnvalue_4 (DynamicMesh|Reset _returnvalue))
      (Class|GeometryScriptLibraryMeshPrimitiveFunctions|AppendSphereBox :TargetMesh _returnvalue_4 :Debug 0))))